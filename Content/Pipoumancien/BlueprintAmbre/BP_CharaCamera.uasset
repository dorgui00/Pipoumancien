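; BP_CharaCamera is a camera pawn, apparently a debug prototype, that slides sideways when the T debug key is pressed.
; A timeline lerps from the current location toward a point along the right vector on each update, so movement accumulates.
; Custom events play or reverse the timeline and set a direction flag.
; The toggle between them and a forward movement input are left unwired.
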(event Custom|reverse
  ;[0.15 0.15 0.15 0.5] Lerp
  (Variables|Default|SetexecuteReverse true)
  (bind _newtrack_0 (Timeline|Timeline Reverse)
    (:Update
      (Transformation|SetActorLocation (Math|Vector|Lerp(Vector) (Transformation|GetActorLocation) (+ (Transformation|GetActorLocation) (* (Transformation|GetActorRightVector) 2e+01)) _newtrack_0) false false)
      (Variables|Default|SetNewTime 0.0))))

(event Custom|tim
  ;[0.15 0.15 0.15 0.5] Lerp
  (Variables|Default|SetexecuteReverse false)
  (bind _newtrack_0 (Timeline|Timeline PlayFromStart)
    (:Update
      (Transformation|SetActorLocation (Math|Vector|Lerp(Vector) (Transformation|GetActorLocation) (+ (Transformation|GetActorLocation) (* (Transformation|GetActorRightVector) 2e+01)) _newtrack_0) false false)
      (Variables|Default|SetNewTime 0.0))))

(event Input|KeyboardEvents|DebugKeyT
  (params (Key :type Key%20Structure :default "None") (ActionValue :type Input%20Action%20Value%20Structure))
  (:Pressed
    ;[0.15 0.15 0.15 0.5] Lerp
    (bind _newtrack_0 (Timeline|Timeline Play)
      (:Update
        (Transformation|SetActorLocation (Math|Vector|Lerp(Vector) (Transformation|GetActorLocation) (+ (Transformation|GetActorLocation) (* (Transformation|GetActorRightVector) 2e+01)) _newtrack_0) false false)
        (Variables|Default|SetNewTime 0.0)))))

(fn ConstructionScript)