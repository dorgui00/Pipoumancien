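; Game mode for the Pipoumancien project that cycles the player's view between the cinematic cameras placed in the level.
; On BeginPlay it gathers every CineCameraActor into an array.
; The NextCam event advances an index, intended to wrap to the first camera past the end, and sets the first player controller's view target to a camera from that array.
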(event Custom|NextCam
  (bind _cams (Variables|Default|GetCams))
  (bind _result (Math|Integer|IncrementInt (Variables|Default|GetCurrentCam))
    (:%20%20
      (if (Utilities|Array|IsValidIndex _cams _result)
        _
        (else
          (Variables|Default|SetCurrentCam 0)))
      (Game|Player|SetViewTargetwithBlend (Game|GetPlayerController 0) (Utilities|Array|Get(acopy) _cams _result) 0.0 "VTBlend_Linear" 0.0 false))))

(event EventBeginPlay
  (bind _outactors (Actor|GetAllActorsOfClass "/Script/CinematicCamera.CineCameraActor"))
  (Variables|Default|SetCams _outactors))

(event EventTick
  (params (DeltaSeconds :type Float%20%28single-precision%29)))

(fn ConstructionScript)