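; Skeleton NPC controller that animates a skeleton's wake-up during a melody, with dirt particles at each animation step.
; A timer-chained function steps through the WakeAnims array, setting play rate from total animation length over the melody's summed note Frequency values.
; A failed finish flags the sequence to play backwards step by step on shorter timers, relaunching it if it had already ended.
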(event EventPlayWakeAnim
  ;[0.15 0.15 0.15 0.5] Skeleton Controller
  ;;[0.15 0.15 0.15 0.5] Wake anim
  ;;;[0.15 0.15 0.15 0.5] Play Wake Anim
  ;;;;[0.15 0.15 0.15 0.5] Default Play Anim all the time
  (CallFunction|SetAnimData)
  (CallFunction|FInitWakeAnim)
  (CallFunction|CELaunchWakeAnim))

(event EventFinishWakeAnim
  (params (HasSucceed :type Boolean))
  ;[0.15 0.15 0.15 0.5] Skeleton Controller
  ;;[0.15 0.15 0.15 0.5] Wake anim
  ;;;[0.15 0.15 0.15 0.5] Finish Wake Anim
  (if (not HasSucceed)
    (Variables|Default|SetHasFailed true)
    (bind _result (Math|Integer|DecrementInt (Variables|Default|GetCurrentAnimationIndex))
      (:%20%20
        (Variables|Default|SetCurrent%20Animation%20Index (Math|Integer|Max(Integer) _result))
        (if (Variables|Default|GetHasFinishedPlay)
          (CallFunction|CELaunchWakeAnim))))))

(fn ConstructionScript)

(fn SetMelodyLength
  (for _array_element (.Notes (Utilities|Struct|Break_Skeleton (Class|SkeletonController|GetMyData)))
    ;[0.15 0.15 0.15 0.5] Increment frequencies
    (LocalVariables|SetAllFrequencies (+ (LocalVariables|GetAllFrequencies) (.Frequency (Utilities|Struct|Break_Note _array_element)))))
  ;[0.15 0.15 0.15 0.5] Melody Length
  (Variables|Default|SetMelodyLength (LocalVariables|GetAllFrequencies))
  (return))

(fn SetAnimData
  (CallFunction|SetWakeAnimDuration)
  (CallFunction|SetMelodyLength))

(fn SetWakeAnimDuration
  (for _array_element (Variables|Default|GetWakeAnims)
    (Variables|Default|SetWakeAnimDuration (+ (Animation|GetPlayLength _array_element) (Variables|Default|GetWakeAnimDuration)))))

(fn CELaunchWakeAnim
  (if (Utilities|AnimExists)
    (if (Variables|Default|GetHasFailed)
      ;[0.15 0.15 0.15 0.5] Fail
      (CallFunction|FPlayWake -1.0 1.0)
      (Math|Integer|DecrementInt (Variables|Default|GetCurrentAnimationIndex)
        (:%20%20
          (Utilities|Time|SetTimerbyFunctionName 0 "CE_LaunchWakeAnim" 1.0)))
      (else
        ;[0.15 0.15 0.15 0.5] Success
        (CallFunction|FPlayWake (Utilities|PlayRate) 0.0)
        (Math|Integer|IncrementInt (Variables|Default|GetCurrentAnimationIndex)
          (:%20%20
            (Utilities|Time|SetTimerbyFunctionName 0 "CE_LaunchWakeAnim" 3.5)))))
    (else
      (Variables|Default|SetHasFinishedPlay true))))

(fn FPlayWake
  (params (Rate :type Float%20%28double-precision%29) (Pos :type Float%20%28double-precision%29))
  (bind _skeletalmesh (Variables|Default|GetSkeletalMesh))
  ;[0.15 0.15 0.15 0.5] Play Wake
  (Components|Animation|SetAnimation _skeletalmesh (Utilities|Array|Get(acopy) (Variables|Default|GetWakeAnims) (Variables|Default|GetCurrentAnimationIndex)))
  (Components|Animation|SetPosition _skeletalmesh Pos true)
  (Components|Timeline|SetPlayRate (Variables|Default|GetSkeletalMesh) Rate)
  (Audio|Components|Audio|Play (Variables|Default|GetSkeletalMesh) false)
  ;;[0.15 0.15 0.15 0.5] VFX
  (Niagara|SpawnSystematLocation "/Game/Pipoumancien/FX/NS_Dirt_Particles.NS_Dirt_Particles" (Transformation|GetActorLocation) "0, 0, 0" (* (Math|Vector|MakeVector 1.0 1.0 1.0) 2.0)))

(fn FInitWakeAnim
  ;[0.15 0.15 0.15 0.5] Init Wake Anim
  (Variables|Default|SetHasFailed false)
  (Variables|Default|SetCurrentAnimationIndex 0)
  (Variables|Default|SetHasFinishedPlay false))