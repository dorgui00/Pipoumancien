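; BPAIV3 is an NPC that wanders continuously from BeginPlay by moving to random reachable points around its current location.
; A self-restarting custom event picks each point and runs AI MoveTo, pausing after arrival or retrying almost immediately on failure.
; Walk and idle animations play directly on the mesh at each state change.
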(event Custom|CE_MoveNPC
  (Components|Animation|PlayAnimation (Variables|Character|GetMesh) "/Game/Characters/Mannequins/Animations/Quinn/MF_Walk_Fwd.MF_Walk_Fwd" true)
  (bind _output_get (Variables|Default|SetRandom%20Location (.RandomLocation (AI|Navigation|GetRandomReachablePointinRadius (Transformation|GetActorLocation) 7e+02 0 0))))
  (AI|AIMoveTo self _output_get 0 1e+01 false
    (:OnSuccess
      (Components|Animation|PlayAnimation (Variables|Character|GetMesh) "/Game/Characters/Mannequins/Animations/Manny/MM_Idle.MM_Idle" false)
      (Utilities|FlowControl|Delay 2.0)
      (CallFunction|CEMoveNPC))
    (:OnFail
      (Components|Animation|PlayAnimation (Variables|Character|GetMesh) "/Game/Characters/Mannequins/Animations/Manny/MM_Idle.MM_Idle" false)
      (Utilities|FlowControl|Delay 0.1)
      (CallFunction|CEMoveNPC))))

(event EventBeginPlay
  (CallFunction|CEMoveNPC))

(fn ConstructionScript)