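; Scripted dog actor, named as a fake dog for the trailer, that walks to a target and can show or hide a stick.
; CE_MoveChara runs AI MoveTo toward Target, directly playing a looping walk animation while moving and idle on success or failure.
; F_ToggleStick flips the stick mesh's activation and visibility, also activating the Niagara notes effect when shown, without deactivating it when hidden.
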(event Custom|CE_MoveChara
  ;[0.15 0.15 0.15 0.5] Move Chara
  (AI|AIMoveTo self "0, 0, 0" (Variables|Default|GetTarget) 5e+01 false
    (:then
      (bind _asaicontroller (Utilities|Casting|CastToAIController (Pawn|GetController)))
      (if (Utilities|Enum|Equal(Enum) (Class|AIController|GetMoveStatus _asaicontroller) "Moving")
        ;;[0.15 0.15 0.15 0.5] Walk
        (Components|Animation|PlayAnimation (Variables|Default|GetDog) "/Game/Pipoumancien/chara/chien/anim/ChienAnimWalk_Anim.ChienAnimWalk_Anim" true)))
    (:OnSuccess
      ;;[0.15 0.15 0.15 0.5] Idle
      (Components|Animation|PlayAnimation (Variables|Default|GetDog) "/Game/Pipoumancien/chara/chien/anim/ChienAnimIdle_Anim.ChienAnimIdle_Anim" true :!label _label))
    (:OnFail
      (goto _label))))

(fn ConstructionScript)

(fn FToggleStick
  ;[0.15 0.15 0.15 0.5] Set Stick
  (if (Variables|Default|GetStickIsActive)
    ;;[0.15 0.15 0.15 0.5] Deactivate
    (Variables|Default|SetStickIsActive false)
    ;;;[0.15 0.15 0.15 0.5] Stick
    (Components|Activation|Deactivate (Variables|Default|GetSkM_Stick))
    (Rendering|SetVisibility (Variables|Default|GetSkM_Stick) false true)
    (else
      ;;[0.15 0.15 0.15 0.5] Activate stick
      (Variables|Default|SetStickIsActive true)
      ;;;[0.15 0.15 0.15 0.5] Stick
      (Components|Activation|Activate (Variables|Default|GetSkM_Stick) false)
      (Rendering|SetVisibility (Variables|Default|GetSkM_Stick) true true)
      ;;;[0.15 0.15 0.15 0.5] Notes
      (Components|Activation|Activate (Variables|Default|GetNiagaraNotes) false))))