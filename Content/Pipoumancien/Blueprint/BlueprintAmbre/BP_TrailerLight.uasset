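; Trailer helper Blueprint that switches on the house lights of a scene one after another.
; On BeginPlay it collects actors tagged "HouseLight" into an array of Point Lights.
; CE_TurnOnLights starts a timer-driven chain in which each step sets a light's intensity, makes it visible, then schedules itself for the next index until the array ends.
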(event Custom|CE_TurnOnLights
  ;[0.15 0.15 0.15 0.5] Turn on light one by one
  (CallFunction|CETurnonNextLight1))

(event EventBeginPlay
  ;[0.15 0.15 0.15 0.5] Fill HouseLights Array
  (bind _outactors (Actor|GetAllActorswithTag "HouseLight"))
  (for _array_element _outactors
    (bind _aspoint_light (Utilities|Casting|CastToPointLight _array_element))
    (Utilities|Array|Add (Variables|Default|GetHouseLights) _aspoint_light)))

(fn ConstructionScript)

(fn CETurnonNextLight1
  (bind _houselights (Variables|Default|GetHouseLights))
  (bind _lightindex (Variables|Default|GetLightIndex))
  (bind _output (Utilities|Array|Get(acopy) _houselights _lightindex))
  ;[0.15 0.15 0.15 0.5] Turn On next Light
  ;;[0.15 0.15 0.15 0.5] turn on
  (Rendering|Components|Light|SetIntensity (Variables|/Script/Engine.Light|GetLightComponent _output) (Variables|Default|GetIntensity))
  (Rendering|SetVisibility (Variables|/Script/Engine.Actor|GetRootComponent _output) true false)
  ;;[0.15 0.15 0.15 0.5] Recurrence
  (Math|Integer|IncrementInt (Variables|Default|GetLightIndex)
    (:%20%20
      (if (<= (Variables|Default|GetLightIndex) (- (Utilities|Array|Length (Variables|Default|GetHouseLights)) 1))
        (Utilities|Time|SetTimerbyFunctionName 0 "CE_TurnOnNextLight1" (Variables|Default|GetTimer))))))