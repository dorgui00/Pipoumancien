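; Interactable actor that moves once to a preset end position and rotation when Interact or the CE_Test event fires.
; The first trigger sets the targets from a world-space EndPosition offset and an absolute EndRotation.
; Tick interpolates toward them with constant-interp nodes, dividing rotation speed by the remaining quaternion angular distance.
; The construction script draws debug arrows previewing the end offset and rotation.
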(event Custom|CE_Test
  (if (not (Variables|Default|GetbHasInteracted))
    (Variables|Default|SetbHasInteracted true)
    (Variables|Default|SetTarget%20Position (+ (Transformation|GetActorLocation) (Variables|Default|GetEnd%20Position)))
    (Variables|Default|SetTargetRotation (Variables|Default|GetEndRotation))))

(event EventBeginPlay
  (Variables|Default|SetTarget%20Position (Transformation|GetActorLocation))
  (Variables|Default|SetTargetRotation (Transformation|GetActorRotation)))

(event EventTick
  (params (DeltaSeconds :type Float%20%28single-precision%29))
  (bind _returnvalue (Transformation|GetActorRotation))
  (bind _targetrotation (Variables|Default|GetTargetRotation))
  (if (or (Utilities|Operators|NotEqual(!=) (Transformation|GetActorLocation) (Variables|Default|GetTarget%20Position) 1.0) (Utilities|Operators|NotEqual(!=) (Transformation|GetActorRotation) (Variables|Default|GetTargetRotation) 1.0))
    (Transformation|SetActorLocationAndRotation (Math|Interpolation|VInterptoConstant (Transformation|GetActorLocation) (Variables|Default|GetTarget%20Position) DeltaSeconds (Variables|Default|GetInterp%20Speed)) (Class|KismetMathLibrary|RInterptoConstant _returnvalue _targetrotation DeltaSeconds (/ (/ (Variables|Default|GetInterp%20Speed) (Class|KismetMathLibrary|QuatAngularDistance (Math|Conversions|ToQuaternion(Rotator) _returnvalue) (Math|Conversions|ToQuaternion(Rotator) _targetrotation))) 2.0)))))

(event EventInteract
  (if (not (Variables|Default|GetbHasInteracted))
    (Variables|Default|SetbHasInteracted true)
    (Variables|Default|SetTarget%20Position (+ (Transformation|GetActorLocation) (Variables|Default|GetEnd%20Position)))
    (Variables|Default|SetTargetRotation (Variables|Default|GetEndRotation))))

(fn ConstructionScript
  (bind _returnvalue (Transformation|GetActorLocation))
  (Rendering|Debug|DrawDebugArrow (Transformation|GetActorLocation) (+ (Transformation|GetActorLocation) (Variables|Default|GetEnd%20Position)) 32.0 "(R=1.000000,G=0.009211,B=0.000000,A=1.000000)" 5.0 0.0)
  (Rendering|Debug|DrawDebugArrow _returnvalue (+ _returnvalue (* (Math|Vector|RotateVector (Transformation|GetActorForwardVector) (Variables|Default|GetEndRotation)) 1e+02)) 32.0 "(R=0.141643,G=0.000000,B=1.000000,A=1.000000)" 5.0 0.0))