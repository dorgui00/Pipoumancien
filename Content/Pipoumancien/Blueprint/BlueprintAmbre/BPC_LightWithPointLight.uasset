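; Interactable light Blueprint that switches its SpotLight component on and off.
; BeginPlay sets the starting intensity to full or zero from IsLitUp.
; Interact and CE_Test share a FlipFlop that alternates between full and zero intensity.
; The FlipFlop ignores IsLitUp and always turns the light on first, so a light that starts lit shows no change on the first toggle.
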(event Custom|CE_Test
  (bind _spotlight (Variables|Default|GetSpotLight))
  (Utilities|FlowControl|FlipFlop
    (:A
      (Rendering|Components|Light|SetIntensity _spotlight 4e+04))
    (:B
      (Rendering|Components|Light|SetIntensity _spotlight 0.0))))

(event EventBeginPlay
  (Rendering|Components|Light|SetIntensity (Variables|Default|GetSpotLight) (Math|Float|SelectFloat 4e+04 0.0 (Variables|Light|GetbIsLitUp))))

(event EventInteract
  (bind _spotlight (Variables|Default|GetSpotLight))
  (Utilities|FlowControl|FlipFlop
    (:A
      (Rendering|Components|Light|SetIntensity _spotlight 4e+04))
    (:B
      (Rendering|Components|Light|SetIntensity _spotlight 0.0))))

(fn ConstructionScript
  (|CallParentFunction))