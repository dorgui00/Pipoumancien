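; Test Blueprint for a skeleton wake-up animation split into four parts.
; Each part has a custom event that sets the mesh play rate and plays its animation once, and BeginPlay triggers the first after a short delay.
; The length-based delays meant to chain the parts into a looping walk are disconnected, so only the first part is triggered here.
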(event Custom|CE_Part4
  (params (PlayRate :type Float%20%28double-precision%29))
  (bind _mesh (Variables|Character|GetMesh))
  ;[0.15 0.15 0.15 0.5] Part 4
  (Components|Timeline|SetPlayRate _mesh PlayRate)
  (Components|Animation|PlayAnimation _mesh "/Game/Pipoumancien/chara/squelette/anim/Wake/SqueletteAnimWake_Part4.SqueletteAnimWake_Part4" false))

(event Custom|CE_Part3
  (params (PlayRate :type Float%20%28double-precision%29))
  (bind _mesh (Variables|Character|GetMesh))
  ;[0.15 0.15 0.15 0.5] Part 3
  (Components|Timeline|SetPlayRate _mesh PlayRate)
  (Components|Animation|PlayAnimation _mesh "/Game/Pipoumancien/chara/squelette/anim/Wake/SqueletteAnimWake_Part3.SqueletteAnimWake_Part3" false))

(event Custom|CE_Part2
  (params (PlayRate :type Float%20%28double-precision%29))
  (bind _mesh (Variables|Character|GetMesh))
  ;[0.15 0.15 0.15 0.5] Part 2
  (Components|Timeline|SetPlayRate _mesh PlayRate)
  (Components|Animation|PlayAnimation _mesh "/Game/Pipoumancien/chara/squelette/anim/Wake/SqueletteAnimWake_Part2.SqueletteAnimWake_Part2" false))

(event Custom|CE_Part1
  (params (PlayRate :type Float%20%28double-precision%29))
  (bind _mesh (Variables|Character|GetMesh))
  ;[0.15 0.15 0.15 0.5] Part 1
  (Components|Timeline|SetPlayRate _mesh PlayRate)
  (Components|Animation|PlayAnimation _mesh (Variables|Default|GetPart01) false))

(event EventBeginPlay
  (Utilities|FlowControl|Delay 2.0)
  (CallFunction|CEPart1 1.0))

(fn ConstructionScript)