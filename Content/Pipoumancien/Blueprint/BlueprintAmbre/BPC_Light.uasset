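; BPC_Light is an interactable light that toggles the glow of its sphere's glass material.
; On BeginPlay it creates a dynamic instance of M_verre on the sphere and sets its intensity from IsLitUp.
; Interact and the CE_Test event share a FlipFlop that alternates intensity between on and off.
; The FlipFlop ignores IsLitUp, so the first toggle always switches the glow on.
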(event Custom|CE_Test
  (bind _dmi_verre (Variables|Default|GetDMI%20Verre))
  (bind _intensityparamname (Variables|Default|GetIntensityParamName))
  (Utilities|FlowControl|FlipFlop
    (:A
      (Rendering|Material|SetScalarParameterValue _dmi_verre _intensityparamname 1e+02 :!class /Script/Engine.MaterialInstanceDynamic))
    (:B
      (Rendering|Material|SetScalarParameterValue _dmi_verre _intensityparamname 0.0 :!class /Script/Engine.MaterialInstanceDynamic))))

(event EventBeginPlay
  (bind _returnvalue (Rendering|Material|CreateDynamicMaterialInstance (Variables|Default|GetSphere) 2 "/Game/Pipoumancien/Assets/Environement/M_verre.M_verre" "VerreDynamic" :!class /Script/Engine.PrimitiveComponent))
  (bind _output_get (Variables|Default|SetDMI%20Verre _returnvalue))
  (Rendering|Material|SetScalarParameterValue _output_get (Variables|Default|GetIntensityParamName) (Math|Float|SelectFloat 1e+02 0.0 (Variables|Light|GetbIsLitUp)) :!class /Script/Engine.MaterialInstanceDynamic))

(event EventInteract
  (bind _dmi_verre (Variables|Default|GetDMI%20Verre))
  (bind _intensityparamname (Variables|Default|GetIntensityParamName))
  (Utilities|FlowControl|FlipFlop
    (:A
      (Rendering|Material|SetScalarParameterValue _dmi_verre _intensityparamname 1e+02 :!class /Script/Engine.MaterialInstanceDynamic))
    (:B
      (Rendering|Material|SetScalarParameterValue _dmi_verre _intensityparamname 0.0 :!class /Script/Engine.MaterialInstanceDynamic))))

(fn ConstructionScript
  (|CallParentFunction))