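; Scripted stand-in Necromancer, apparently for trailer shots, that walks to a target alone or together with the tagged fake dog found on BeginPlay.
; Move events drive AIMoveTo and play walk or idle animations directly on the mesh.
; While moving, Tick uses a Delay to pace footsteps, tracing down to pick snow, dirt, grass or road sounds by physical material.
; A separate function toggles the flute mesh and its Niagara notes.
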(event Custom|CE_MoveChara
  ;[0.15 0.15 0.15 0.5] Move Chara
  (AI|AIMoveTo self "0, 0, 0" (Variables|Default|GetTarget) 5e+01 false
    (:then
      (bind _asaicontroller (Utilities|Casting|CastToAIController (Pawn|GetController)))
      (if (Utilities|Enum|Equal(Enum) (Class|AIController|GetMoveStatus _asaicontroller) "Moving")
        (Variables|Default|SetbMoving true)
        (Components|Animation|PlayAnimation (Variables|Default|GetNecro) "/Game/Pipoumancien/chara/necromancien/Anim_8/NecromancienAnimWalk_08_Anim_Armature_Armature_001_Armature_ArmatureAction.NecromancienAnimWalk_08_Anim_Armature_Armature_001_Armature_ArmatureAction" true)
        (else
          (Variables|Default|SetbMoving false))))
    (:OnSuccess
      ;;[0.15 0.15 0.15 0.5] Idle
      (Components|Animation|PlayAnimation (Variables|Default|GetNecro) "/Game/Pipoumancien/chara/necromancien/Anim_8/NecromancienAnimIdle_08_Anim.NecromancienAnimIdle_08_Anim" true :!label _label)
      (Variables|Default|SetbMoving false))
    (:OnFail
      (goto _label))))

(event Custom|CE_MoveBoth
  ;[0.15 0.15 0.15 0.5] Move At the same time
  (Default|CEMoveChara (Variables|Default|GetDog))
  (CallFunction|CEMoveChara))

(event EventTick
  (params (DeltaSeconds :type Float%20%28single-precision%29))
  (bind _necro (Variables|Default|GetNecro))
  (bind _returnvalue (Transformation|GetWorldLocation _necro))
  (if (Variables|Default|GetbMoving)
    (Utilities|FlowControl|Delay (Variables|Default|GetFootstep_Interval))
    (bind _outhit (Collision|LineTraceByChannel _returnvalue (- _returnvalue "0.000000,0.000000,50.000000") "TraceTypeQuery1" false 0 "None"))
    (if (== (.PhysMat (Collision|BreakHitResult _outhit)) (Variables|PhysMat|GetSnowMat))
      (Variables|Sounds|SetSoundToPlay_Walk (Variables|Sounds|GetSnowSound))
      (Audio|PlaySoundatLocation (Variables|Sounds|GetSoundToPlay_Walk) (Transformation|GetWorldLocation (Variables|Default|GetNecro)) "0, 0, 0" 1.0 1.0 0.0 0 0 0 0 :!label _label)
      (elif (== (.PhysMat (Collision|BreakHitResult _outhit)) (Variables|PhysMat|GetDirtMat))
        (Variables|Sounds|SetSoundToPlay_Walk (Variables|Sounds|GetDirtSound))
        (goto _label)
        (elif (== (.PhysMat (Collision|BreakHitResult _outhit)) (Variables|PhysMat|GetGrassMat))
          (Variables|Sounds|SetSoundToPlay_Walk (Variables|Sounds|GetGrassSound))
          (goto _label)
          (elif (== (.PhysMat (Collision|BreakHitResult _outhit)) (Variables|PhysMat|GetRoadMat))
            (Variables|Sounds|SetSoundToPlay_Walk (Variables|Sounds|GetRoadSound))
            (goto _label)))))))

(event EventBeginPlay
  ;[0.15 0.15 0.15 0.5] Get Dog
  (bind _outactors (Actor|GetAllActorswithTag "FakeDog"))
  (bind _asbp_trailer_fake_dog (Utilities|Casting|CastToBP_TrailerFakeDog (Utilities|Array|Get(acopy) _outactors)))
  (Variables|Default|SetDog _asbp_trailer_fake_dog))

(fn ConstructionScript)

(fn FToggleFlute
  ;[0.15 0.15 0.15 0.5] Set Flute
  (if (Variables|Default|GetIsFluteActive)
    ;;[0.15 0.15 0.15 0.5] Deactivate
    (Variables|Default|SetIsFluteActive false)
    ;;;[0.15 0.15 0.15 0.5] Flute
    (Components|Activation|Deactivate (Variables|Default|GetSkM_Flute))
    (Rendering|SetVisibility (Variables|Default|GetSkM_Flute) false true)
    ;;;[0.15 0.15 0.15 0.5] Notes
    (Components|Activation|Deactivate (Variables|Default|GetNiagaraNotes))
    (else
      ;;[0.15 0.15 0.15 0.5] Activate flute
      (Variables|Default|SetIsFluteActive true)
      ;;;[0.15 0.15 0.15 0.5] Flute
      (Components|Activation|Activate (Variables|Default|GetSkM_Flute) false)
      (Rendering|SetVisibility (Variables|Default|GetSkM_Flute) true true)
      ;;;[0.15 0.15 0.15 0.5] Notes
      (Components|Activation|Activate (Variables|Default|GetNiagaraNotes) false))))