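; Interactable trunk actor that moves and rotates once to a preset end pose when first interacted with.
; Interaction offsets the target position by EndPosition and sets the absolute EndRotation, guarded by HasInteracted.
; Tick interpolates toward both targets, deriving rotation speed from InterpSpeed and the remaining quaternion angular distance.
; As rotation nears its target during movement, a DoOnce activates the Niagara effect and zeroes its world rotation.
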(event Custom|CustomEvent
  (if (not (Variables|Default|GetbHasInteracted))
    (Variables|Default|SetbHasInteracted true)
    (Variables|Default|SetTarget%20Position (+ (Transformation|GetActorLocation) (Variables|Default|GetEnd%20Position)))
    (Variables|Default|SetTargetRotation (Variables|Default|GetEndRotation))))

(event EventBeginPlay
  (Variables|Default|SetTarget%20Position (Transformation|GetActorLocation))
  (Variables|Default|SetTargetRotation (Transformation|GetActorRotation)))

(event EventTick
  (params (DeltaSeconds :type Float%20%28single-precision%29))
  (bind _returnvalue (Transformation|GetActorRotation))
  (bind _targetrotation (Variables|Default|GetTargetRotation))
  (bind _niagara (Variables|Default|GetNiagara))
  (bind _returnvalue_2 (Math|Conversions|ToQuaternion(Rotator) _returnvalue))
  (bind _returnvalue_3 (Math|Conversions|ToQuaternion(Rotator) _targetrotation))
  (if (or (Utilities|Operators|NotEqual(!=) (Transformation|GetActorLocation) (Variables|Default|GetTarget%20Position) 1.0) (Utilities|Operators|NotEqual(!=) (Transformation|GetActorRotation) (Variables|Default|GetTargetRotation) 1.0))
    (Transformation|SetActorLocationAndRotation (Math|Interpolation|VInterptoConstant (Transformation|GetActorLocation) (Variables|Default|GetTarget%20Position) DeltaSeconds (Variables|Default|GetInterp%20Speed)) (Class|KismetMathLibrary|RInterptoConstant _returnvalue _targetrotation DeltaSeconds (/ (/ (Variables|Default|GetInterp%20Speed) (Class|KismetMathLibrary|QuatAngularDistance _returnvalue_2 _returnvalue_3)) 2.0)))
    (if (Utilities|Operators|EqualEqual _returnvalue_2 _returnvalue_3 0.1)
      (Utilities|FlowControl|DoOnce false
        (:Completed
          (Components|Activation|SetActive _niagara true false)
          (Transformation|SetWorldRotation _niagara "0, 0, 0" false false))))))

(event EventInteract
  (if (not (Variables|Default|GetbHasInteracted))
    (Variables|Default|SetbHasInteracted true)
    (Variables|Default|SetTarget%20Position (+ (Transformation|GetActorLocation) (Variables|Default|GetEnd%20Position)))
    (Variables|Default|SetTargetRotation (Variables|Default|GetEndRotation))))

(fn ConstructionScript
  (|CallParentFunction))